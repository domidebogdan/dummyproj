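; Orbit camera pawn for the ArchViz Explorer, driven by mouse and touch, that also creates the master menu widget on BeginPlay.
; Held mouse or touch drags rotate the spring arm, with an optional pitch clamp applied to actor rotation.
; Wheel and pinch set a target arm length scaled by a distance-based curve, which Tick eases toward at curve-driven speed.
; Focus event uses a timeline to blend the actor to a new location and rotation.
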(event `Key|LeftMouseButton`
  (params (Key :type "Key Structure"))
  ;[1 1 1] Check mouse button hold
  (:`Pressed`
    (`KismetSystemLibrary.Delay` 0.2)
    (if (`PlayerController.IsInputKeyDown` (`GameplayStatics.GetPlayerController` 0) "LeftMouseButton")
      (set `self.Hold` true)))
  (:`Released`
    (set `self.Hold` false)))

(event `Key|Touch1` :consume false
  (params (Key :type "Key Structure"))
  ;[0.5 1 0.5] Check Touch Finger Count
  (:`Pressed`
    (set `self.Touch_F1_Pressed` true)
    (set `self.Touch_F_Count` (+ (`KismetMathLibrary.Conv_BoolToInt` (`self.Touch_F1_Pressed`)) (`KismetMathLibrary.Conv_BoolToInt` (`self.Touch_F2_Pressed`))) :!label _label))
  (:`Released`
    (set `self.Touch_F1_Pressed` false)
    (goto _label)))

(event `Key|Touch2` :consume false
  (params (Key :type "Key Structure"))
  ;[0.5 1 0.5] Check Touch Finger Count
  (:`Pressed`
    (set `self.Touch_F2_Pressed` true)
    (goto _label))
  (:`Released`
    (set `self.Touch_F2_Pressed` false)
    (goto _label)))

(event `InputTouch`
  (params (Location :type "Vector Structure") (FingerIndex :type "ETouchIndex Enum"))
  (bind _returnvalue (`GameplayStatics.GetPlayerController` 0))
  (bind _pitchlimit_min (`self.PitchLimit_Min`))
  (bind _pitchlimit_max (`self.PitchLimit_Max`))
  (bind _pitch (.pitch (`self.K2_GetActorRotation`)))
  (bind (_locationx _locationy _biscurrentlypressed) (`PlayerController.GetInputTouchState` _returnvalue "Touch1"))
  (bind (_locationx_2 _locationy_2) (`PlayerController.GetInputTouchState` (`GameplayStatics.GetPlayerController` 0) FingerIndex))
  (bind (_locationx_3 _locationy_3 _biscurrentlypressed_2) (`PlayerController.GetInputTouchState` _returnvalue "Touch2"))
  (bind _returnvalue_2 (< _pitch _pitchlimit_min))
  (bind _returnvalue_3 (or _biscurrentlypressed _biscurrentlypressed_2))
  (bind (_returnvalue_x _returnvalue_y) (`KismetMathLibrary.BreakVector2D` (* (* (- (`KismetMathLibrary.MakeVector2D` _locationx_2 _locationy_2) (`self.Touch_Location_Start`)) (`self.Rotation_Speed_Touch`)) (`GameplayStatics.GetWorldDeltaSeconds`))))
  ;[0.5 1 0.5] Touch Rotation
  (:`Pressed`
    ;[0.5 1 0.5] Check touch hold
    (if (and _biscurrentlypressed _biscurrentlypressed_2)
      (set `self.Hold` true :!label _label_2)
      (else
        (`KismetSystemLibrary.Delay` 0.3)
        (if _returnvalue_3
          (goto _label_2)))))
  (:`Released`
    (`KismetSystemLibrary.Delay` 0.2)
    (if _returnvalue_3
      (set `self.Hold` true)
      (else
        (set `self.Hold` false))))
  (:`Moved`
    (if (`self.InputLocked`)
      _
      (elif (< (`self.Touch_F_Count`) 2)
        (set `self.Touch_Location_Start` (`KismetMathLibrary.MakeVector2D` Location_X Location_Y))
        (`SceneComponent.K2_AddRelativeRotation` (`self.SpringArm1`) (`KismetMathLibrary.MakeRotator` 0.0 (* _returnvalue_y -1.0) _returnvalue_x) false false)
        ;[1 1 1] Limit Pitch Rotation
        (if (`self.PitchLimit`) :!label _label_3
          (if (or _returnvalue_2 (> _pitch _pitchlimit_max))
            (`self.K2_SetActorRotation` (`KismetMathLibrary.MakeRotator` 0.0 (`KismetMathLibrary.SelectFloat` _pitchlimit_min _pitchlimit_max _returnvalue_2) (.yaw (`self.K2_GetActorRotation`))))))))))

(event `self.ReceiveBeginPlay`
  (`|ExecutionSequence`
    (:`then_0`
      ;[1 1 1] Show mouse cursor at BeginPlay
      (set `PlayerController.bShowMouseCursor` true (`GameplayStatics.GetPlayerController` 0))
      (set `self.TargetArmLength_New` (`SpringArmComponent.TargetArmLength` (`self.SpringArm1`))))
    (:`then_1`
      ;[1 1 1] Add "BP_MasterWidget" to viewport and store it
      (bind _returnvalue (`|CreateWidget` "/Game/ArchVizExplorer/Blueprints/Widgets/BP_MasterMenu_Widget.BP_MasterMenu_Widget_C"))
      (bind _output_get (set `self.BP_MasterMenu` _returnvalue))
      (`UserWidget.AddToViewport` _output_get 0))))

(event `InputAxisKey|MouseX`
  (params (AxisValue :type "Float (single-precision)"))
  ;[1 1 1] Rotation
  (if (`self.InputLocked`)
    _
    (elif (`self.Hold`)
      (`SceneComponent.K2_AddRelativeRotation` (`self.SpringArm1`) (`KismetMathLibrary.MakeRotator` 0.0 0.0 (* AxisValue (`self.RotationSpeed_Mouse`))) false false)
      (goto _label_3))))

(event `InputAxisKey|MouseY`
  (params (AxisValue :type "Float (single-precision)"))
  ;[1 1 1] Rotation
  (if (`self.InputLocked`)
    _
    (elif (`self.Hold`)
      (`SceneComponent.K2_AddRelativeRotation` (`self.SpringArm1`) (`KismetMathLibrary.MakeRotator` 0.0 (* AxisValue (`self.RotationSpeed_Mouse`))) false false)
      (goto _label_3))))

(event `InputAxis|PinchGesture`
  (params (AxisValue :type "Float (single-precision)"))
  (bind _pinch_threshold (`self.Pinch_Threshold`))
  (bind _targetarmlength (`SpringArmComponent.TargetArmLength` (`self.SpringArm1`)))
  (bind _returnvalue (* (* (`KismetMathLibrary.FClamp` (- AxisValue 1.0) -0.5 0.5) -1.0) (`CurveFloat.GetFloatValue` (`self.Zoom_Intensity_Curve`) (`KismetMathLibrary.NormalizeToRange` _targetarmlength (`self.SpringArm_Length_Min`) (`self.SpringArm_Length_Max`))) (`self.Pinch_Speed_Multiply`)))
  (bind _returnvalue_2 (+ _targetarmlength _returnvalue))
  (bind _returnvalue_3 (+ _targetarmlength _returnvalue))
  ;[0.5 1 0.5] Touch Zoom / Pinch
  (`/Engine/EditorBlueprintResources/StandardMacros.Gate` true :!label _label_4
    (:`Exit`
      (if (not (== AxisValue (`self.Pinch_AxisValue`)))
        (set `self.Pinch_AxisValue` AxisValue)
        (if (> AxisValue 0.0)
          ;;[1 1 1] Zoom In / Open fingers
          (`/Engine/EditorBlueprintResources/StandardMacros.CompareFloat` _returnvalue_2 _pinch_threshold
            (:`>`
              (set `self.TargetArmLength_New` _returnvalue_2)))
          (else
            ;;[1 1 1] Zoom Out / Close fingers
            (`/Engine/EditorBlueprintResources/StandardMacros.CompareFloat` _returnvalue_3 (* _pinch_threshold -1.0)
              (:`<`
                (set `self.TargetArmLength_New` _returnvalue_3)))))))))

(event `Key|Gesture_Pinch`
  (params (Key :type "Key Structure"))
  ;[0.5 1 0.5] Touch Zoom / Pinch
  (:`Pressed`
    (set `self.Hold` true)
    (goto _label_4 :!via `Open`))
  (:`Released`
    (goto _label_4 :!via `Close`)))

(event `Focus`
  (bind (_returnvalue_roll _returnvalue_pitch _returnvalue_yaw) (`KismetMathLibrary.BreakRotator` (`self.K2_GetActorRotation`)))
  (`|ExecutionSequence`
    (:`then_0`
      ;[1 1 1] Store Current Location and Rotation
      (set `self.Location_Current` (`self.K2_GetActorLocation`))
      (set `self.Pitch_Current` _returnvalue_pitch)
      (set `self.Yaw_Current` _returnvalue_yaw))
    (:`then_1`
      (`TimelineComponent.SetPlayRate` (`self.Timeline_Focus_Animation`) (`self.Focus_Animation_PlayRate`))
      ;[1 1 1] Location and Rotation animation
      (bind (_direction _lerp) (`Timeline|Timeline_Focus_Animation` :!via `PlayFromStart`) ; Focus animation
        (:`Update`
          (`self.K2_SetActorLocation` (`KismetMathLibrary.VLerp` (`self.Location_Current`) (`self.Location_New`) _lerp))
          (`self.K2_SetActorRotation` (`KismetMathLibrary.RLerp` (`KismetMathLibrary.MakeRotator` 0.0 (`self.Pitch_Current`) (`self.Yaw_Current`)) (`KismetMathLibrary.MakeRotator` 0.0 (`self.Pitch_New`) (`self.Yaw_New`)) _lerp true)))))))

(event `Key|MouseScrollUp`
  (params (Key :type "Key Structure"))
  (bind _targetarmlength (`SpringArmComponent.TargetArmLength` (`self.SpringArm1`)))
  ;[1 1 1] Zoom In/Out
  (:`Pressed`
    (if (not (`self.InputLocked`))
      (set `self.TargetArmLength_New` (`KismetMathLibrary.FClamp` (- _targetarmlength (* (`CurveFloat.GetFloatValue` (`self.Zoom_Intensity_Curve`) (`KismetMathLibrary.NormalizeToRange` _targetarmlength (`self.SpringArm_Length_Min`) (`self.SpringArm_Length_Max`))) (`self.ZoomSpeed_Mouse`))) (`self.SpringArm_Length_Min`) (`self.SpringArm_Length_Max`))))))

(event `Key|MouseScrollDown`
  (params (Key :type "Key Structure"))
  (bind _targetarmlength (`SpringArmComponent.TargetArmLength` (`self.SpringArm1`)))
  ;[1 1 1] Zoom In/Out
  (:`Pressed`
    (if (not (`self.InputLocked`))
      (set `self.TargetArmLength_New` (`KismetMathLibrary.FClamp` (+ _targetarmlength (* (`CurveFloat.GetFloatValue` (`self.Zoom_Intensity_Curve`) (`KismetMathLibrary.NormalizeToRange` _targetarmlength (`self.SpringArm_Length_Min`) (`self.SpringArm_Length_Max`))) (`self.ZoomSpeed_Mouse`))) (`self.SpringArm_Length_Min`) (`self.SpringArm_Length_Max`))))))

(event `self.ReceiveTick`
  (params (DeltaSeconds :type "Float (single-precision)"))
  (bind _springarm1 (`self.SpringArm1`))
  (bind _targetarmlength (`SpringArmComponent.TargetArmLength` _springarm1))
  ;[1 0 0] Event Tick
  ;[1 1 1] Smooth zoom when scrolling or when changing SpringArm Length
  (set `SpringArmComponent.TargetArmLength` (`KismetMathLibrary.FInterpTo` _targetarmlength (`self.TargetArmLength_New`) (`GameplayStatics.GetWorldDeltaSeconds`) (`CurveFloat.GetFloatValue` (`self.Zoom_InterpSpeed_Curve`) (`KismetMathLibrary.NormalizeToRange` _targetarmlength (`self.SpringArm_Length_Min`) (`self.SpringArm_Length_Max`)))) _springarm1))

(fn `UserConstructionScript`)